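; BP_Monster is a patrolling enemy that ends the game when the player character touches it.
; Its construction script feeds two relative points, Location01 and Location02, plus a Duration variable into an InterpToMovement component to define its path.
; On overlap with player 0's character, it pauses the game and adds a GameOver widget to the viewport.
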(event EventBeginPlay)

(event EventTick
  (params (DeltaSeconds :type Float%20%28single-precision%29)))

(event Collision|EventActorBeginOverlap
  (params (OtherActor :type Actor%20Object%20Reference))
  (if (== OtherActor (Game|GetPlayerCharacter 0))
    (Game|SetGamePaused true)
    (bind _returnvalue (UserInterface|CreateWidget "/Game/UI/GameOver.GameOver_C"))
    (UserInterface|Viewport|AddtoViewport _returnvalue 0)))

(fn ConstructionScript
  (bind _interptomovement (Variables|Default|GetInterpToMovement))
  (Variables|/Script/Engine.InterpToMovementComponent|SetControlPoints _interptomovement (Utilities|Array|MakeArray (Utilities|Struct|MakeInterpControlPoint (Variables|Default|GetLocation01) true) (Utilities|Struct|MakeInterpControlPoint (Variables|Default|GetLocation02) true)))
  (Variables|/Script/Engine.InterpToMovementComponent|SetDuration _interptomovement (Variables|Default|GetDuration)))